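; BP_TCCharacter is a character Blueprint that displays a player name and a colorable health bar.
; On BeginPlay, the server gets a generated name from TCGameInstance and stores it in PlayerName, whose RepNotify writes it to the NameComponent text.
; A separate event passes a color to the WBP_HealthBar widget inside HealthBarComponent.
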(event EventBeginPlay
  (|CallParentFunction)
  (Networking|SwitchHasAuthority
    (:Authority
      (bind _astcgame_instance (Utilities|Casting|CastToTCGameInstance (Game|GetGameInstance)))
      (bind _returnvalue (Class|TCGameInstance|GeneratePlayerName _astcgame_instance))
      (Variables|TCCharacter|SetPlayerName (Utilities|String|ToString(Text) _returnvalue)))))

(event EventUpdateHeathBarColor
  (params (Color :type Linear%20Color%20Structure%20%28by%20ref%29))
  (bind _aswbp_health_bar (Utilities|Casting|CastToWBP_HealthBar (UserInterface|GetUserWidgetObject (Variables|Default|GetHealthBarComponent))))
  (Default|SetColor _aswbp_health_bar Color))

(fn ConstructionScript)

(fn OnRepPlayerName
  (Rendering|Components|TextRender|SetText (Variables|Default|GetNameComponent) (Utilities|Text|ToText(String) (Variables|TCCharacter|GetPlayerName))))